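; BP_Target is a shootable target that reacts to first-person projectiles and adds to a global hit count.
; On BeginPlay it activates its InterpToMovement component when GI_Global's Difficult flag is set, so targets move in that mode.
; A projectile overlapping TargetCollision is destroyed, plays a party-popper sound and Niagara blood burst, increments TargetsHit in GI_Global, then destroys the target.
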(event `self.ReceiveBeginPlay`
  (bind _asgi_global (cast `/Game/Game/Frazier/Blueprints/GI_Global` (`GameplayStatics.GetGameInstance`)))
  (if (`/Game/Game/Frazier/Blueprints/GI_Global.bDifficult` _asgi_global)
    (`ActorComponent.Activate` (`self.InterpToMovement`) false)))

(event `self.TargetCollision.OnComponentBeginOverlap`
  (params (OverlappedComponent :type "PrimitiveComponent Object Reference") (OtherActor :type "Actor Object Reference") (OtherComp :type "PrimitiveComponent Object Reference") (OtherBodyIndex :type Integer) (bFromSweep :type Boolean) (SweepResult :type "HitResult Structure (by ref)"))
  (bind _returnvalue (`self.K2_GetActorLocation`))
  (bind _asbp_first_person_projectile (cast `/Game/FirstPerson/Blueprints/BP_FirstPersonProjectile` OtherActor))
  (`self.K2_DestroyActor` _asbp_first_person_projectile)
  (`GameplayStatics.PlaySoundAtLocation` "/Game/Game/Frazier/Sounds/A_Party_Popper.A_Party_Popper" _returnvalue (struct) 1.0 1.0 0.0 null null null null)
  (`NiagaraFunctionLibrary.SpawnSystemAtLocation` "/Game/Game/Artin/Particles/NS_BloodBurst.NS_BloodBurst" _returnvalue)
  (bind _asgi_global (cast `/Game/Game/Frazier/Blueprints/GI_Global` (`GameplayStatics.GetGameInstance`)))
  (`/Engine/EditorBlueprintResources/StandardMacros.IncrementInt` (`/Game/Game/Frazier/Blueprints/GI_Global.TargetsHit` _asgi_global)
    (:`  `
      (`self.K2_DestroyActor`))))

(fn `UserConstructionScript`)