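; BP_TargetSpawnManager drives target spawning and ends the game when too many targets accumulate.
; It caches all BP_TargetSpawner actors on BeginPlay, and a Tick timer tells a small random number of randomly picked spawners to spawn a target.
; Each wave shortens the interval down to a floor, then counts live BP_Target actors and opens LV_MainMenu if the limit is reached.
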(event `self.ReceiveBeginPlay`
  (bind _outactors (`GameplayStatics.GetAllActorsOfClass` "/Game/Game/Frazier/Blueprints/BP_TargetSpawner.BP_TargetSpawner_C"))
  (set `self.TargetSpawners` _outactors))

(event `self.ReceiveTick`
  (params (DeltaSeconds :type "Float (single-precision)"))
  (bind _output_get (set `self.CurrentTime` (+ (`self.CurrentTime`) (`GameplayStatics.GetWorldDeltaSeconds`))))
  (if (>= _output_get (`self.SpawnTime`))
    (set `self.CurrentTime` 0.0)
    (for _ (range (+ (`KismetMathLibrary.RandomInteger` 2) 1))
      (`/Game/Game/Frazier/Blueprints/BP_TargetSpawner.SpawnTarget` (`KismetArrayLibrary.Array_Random` (`self.TargetSpawners`))))
    (set `self.SpawnTime` (`KismetMathLibrary.FClamp` (- (`self.SpawnTime`) 0.3) 0.5 10000.0))
    (bind _outactors (`GameplayStatics.GetAllActorsOfClass` "/Game/Game/Frazier/Blueprints/BP_Target.BP_Target_C"))
    (if (>= (`KismetArrayLibrary.Array_Length` _outactors) 10)
      (`GameplayStatics.OpenLevelBySoftObjectPtr` "/Game/Game/Frazier/Levels/LV_MainMenu.LV_MainMenu"))))

(fn `UserConstructionScript`)